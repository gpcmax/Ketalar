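; Player character Blueprint with directional flipbook animation, a mouse-driven cable, health and a pause menu.
; Axis input moves it and picks walk flipbooks, with forward/back taking priority over sideways.
; Holding left mouse attaches the cable to a spawned MouseLocation actor and enables its collision.
; TakeHit reduces health or triggers death animation, fade and game-mode loading; Tick spawns a fading-in low-health sound every frame below the threshold.
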(event `self.ReceiveTick`
  (params (DeltaSeconds :type "Float (single-precision)"))
  (`|ExecutionSequence`
    (:`then_0`
      (if (== (`self.ForwardValue`) 0.0)
        (set `self.MovingForwardOrBackward` false)))
    (:`then_1`
      (if (`self.Dead`)
        _
        (elif (not (> (`KismetMathLibrary.VSize` (`self.GetVelocity`)) 0.0))
          (`PaperFlipbookComponent.SetFlipbook` (`self.Sprite`) "/Game/Assets/Sprites/S_Main_Front_Flipbook.S_Main_Front_Flipbook")
          (set `self.MovingForwardOrBackward` false))))
    (:`then_2`
      (if (< (`self.Health`) 50.0)
        (bind _returnvalue (`GameplayStatics.SpawnSoundAtLocation` "/Game/Sounds/Effects/Player_Low_Health_Cue.Player_Low_Health_Cue" (`SceneComponent.K2_GetComponentLocation` (`self.CapsuleComponent`)) (struct) 1.0 1.0 0.0 null null))
        (`/Engine/EditorBlueprintResources/StandardMacros.IsValid` _returnvalue
          (:`Is Valid`
            (`AudioComponent.FadeIn` _returnvalue 5.0 1.0 0.0)))))))

(event `InputAxis|MoveForward`
  (params (AxisValue :type "Float (single-precision)"))
  (bind _sprite (`self.Sprite`))
  (set `self.ForwardValue` AxisValue)
  (`self.AddMovementInput` (`KismetMathLibrary.GetForwardVector` (`KismetMathLibrary.MakeRotator` 0.0 (.pitch (`self.GetControlRotation`)))) AxisValue)
  (if (== AxisValue 1.0)
    (`PaperFlipbookComponent.SetFlipbook` _sprite "/Game/Assets/AnimAssets/Char/Char_Walk_Back/FB_BackWalk.FB_BackWalk")
    (set `self.MovingForwardOrBackward` true)
    (elif (== AxisValue -1.0)
      (`PaperFlipbookComponent.SetFlipbook` _sprite "/Game/Assets/AnimAssets/Char/Char_WalkForward/frontwalk.frontwalk")
      (set `self.MovingForwardOrBackward` true))))

(event `InputAxis|MoveRight`
  (params (AxisValue :type "Float (single-precision)"))
  (bind _sprite (`self.Sprite`))
  (`self.AddMovementInput` (`KismetMathLibrary.GetRightVector` (`KismetMathLibrary.MakeRotator` 0.0 (.pitch (`self.GetControlRotation`)))) AxisValue)
  (if (`self.MovingForwardOrBackward`)
    _
    (elif (== AxisValue 1.0)
      (`PaperFlipbookComponent.SetFlipbook` _sprite "/Game/Assets/AnimAssets/Char/Char_Walk_SideRight/FB_RightSide.FB_RightSide")
      (elif (== AxisValue -1.0)
        (`PaperFlipbookComponent.SetFlipbook` _sprite "/Game/Assets/AnimAssets/Char/Char_Walk_SideLeft/FB_SideView_Left_Walk.FB_SideView_Left_Walk")))))

(event `self.ReceiveBeginPlay`
  (set `PlayerController.bShowMouseCursor` false (`GameplayStatics.GetPlayerController` 0))
  (bind _returnvalue (`|SpawnActorFromClass` "/Game/Test/MouseLocation.MouseLocation_C" (`KismetMathLibrary.MakeTransform` (0.0 0.0 0.0)) "AlwaysSpawn" "OverrideRootScale" null null))
  (set `self.MouseLoc` _returnvalue)
  (`PrimitiveComponent.SetConstraintMode` (`self.Cable`) "YZPlane"))

(event `Key|LeftMouseButton`
  (params (Key :type "Key Structure"))
  (bind _cable (`self.Cable`))
  (bind _mouseloc (`self.MouseLoc`))
  (bind _cube (`/Game/Test/MouseLocation.Cube` _mouseloc))
  (:`Pressed`
    (`PrimitiveComponent.SetCollisionResponseToAllChannels` _cube "ECR_Overlap")
    (`PrimitiveComponent.SetCollisionResponseToChannel` _cube "ECC_PhysicsBody" "ECR_Block")
    (`CableComponent.SetAttachEndTo` _cable _mouseloc "None" "None"))
  (:`Released`
    (`PrimitiveComponent.SetCollisionResponseToAllChannels` _cube "ECR_Ignore")
    (`CableComponent.SetAttachEndTo` _cable null "None" "None")))

(event `Death`
  (set `self.Dead` true)
  (`MovementComponent.StopMovementImmediately` (`self.CharacterMovement`))
  (set `CharacterMovementComponent.MaxWalkSpeed` 0.0 (`self.CharacterMovement`))
  (`SceneComponent.SetHiddenInGame` (`self.Cable`) true false)
  (`PaperFlipbookComponent.SetFlipbook` (`self.Sprite`) "/Game/Assets/AnimAssets/Char/Char_Death/deathAnim.deathAnim")
  (`KismetSystemLibrary.Delay` (`PaperFlipbookComponent.GetFlipbookLength` (`self.Sprite`)))
  (`PaperFlipbookComponent.SetFlipbook` (`self.Sprite`) "/Game/Assets/AnimAssets/Char/Char_Death/Dead.Dead")
  (bind _returnvalue (`|CreateWidget` "/Game/UI/FadeIn.FadeIn_C" (`GameplayStatics.GetPlayerController` 0)))
  (`UserWidget.AddToViewport` _returnvalue 0)
  (`KismetSystemLibrary.Delay` 5.0)
  (bind _asdungeon_game_mode (cast `/Game/BP/DungeonGameMode` (`GameplayStatics.GetGameMode`)))
  (set `/Game/BP/DungeonGameMode.Loading` true _asdungeon_game_mode))

(event `Key|P`
  (params (Key :type "Key Structure"))
  (:`Pressed`
    (bind _returnvalue (`|CreateWidget` "/Game/UI/UI_Pause.UI_Pause_C" (`GameplayStatics.GetPlayerController` 0)))
    (`UserWidget.AddToViewport` _returnvalue 0)
    (`GameplayStatics.SetGamePaused` true)
    (`WidgetBlueprintLibrary.SetInputMode_UIOnlyEx` (`GameplayStatics.GetPlayerController` 0) null)))

(fn `TakeHit`
  (params (B :type "Float (double-precision)"))
  (if (> (`self.Health`) 0.0)
    (set `self.Health` (- (`self.Health`) B))
    (`GameplayStatics.PlaySound2D` "/Game/Sounds/Effects/PlayerHurt.PlayerHurt" 1.0 1.0 0.0 null null)
    (else
      (`self.Death`))))

(fn `UserConstructionScript`)