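; Flipbook-animated enemy child Blueprint that attacks the player and reports its death to its EnemySpawner, with randomized walk speed set at construction.
; A sphere overlap halts movement and plays a left or right attack flipbook, while side colliders damage the player.
; Die plays death animations and sound, increments the spawner's kill count, then destroys the actor.
; OnDestroyed increments that count again, plus the player's, and removes the spawner array's last entry.
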(event `self.ReceiveBeginPlay`
  (`parent.ReceiveBeginPlay`)
  (add `self.OnDestroyed` (delegate `OnDIe`)))

(event `OnDIe` :!signature `self.OnDestroyed`
  (params (DestroyedActor :type "Actor Object Reference"))
  (bind _enemyspawner (`self.EnemySpawner`))
  (bind _enemyspawner_2 (`self.EnemySpawner`))
  (bind _asbp_player_character (cast `/Game/Test/BP_PlayerCharacter` (`GameplayStatics.GetPlayerCharacter` 0) :!pure true))
  (bind _enemyarray (`/Game/BP/EnemySpawner.EnemyArray` _enemyspawner))
  (`/Engine/EditorBlueprintResources/StandardMacros.IsValid` _enemyspawner
    (:`Is Valid`
      (`KismetArrayLibrary.Array_Remove` _enemyarray (- (`KismetArrayLibrary.Array_Length` _enemyarray) 1))
      (set `/Game/BP/EnemySpawner.EnemyKilled` (+ (`/Game/BP/EnemySpawner.EnemyKilled` _enemyspawner_2) 1) _enemyspawner_2)
      (set `/Game/Test/BP_PlayerCharacter.EnemyKilled` (+ (`/Game/Test/BP_PlayerCharacter.EnemyKilled` _asbp_player_character) 1) _asbp_player_character))))

(event `self.Sphere_0.OnComponentBeginOverlap`
  (params (OverlappedComponent :type "PrimitiveComponent Object Reference") (OtherActor :type "Actor Object Reference") (OtherComp :type "PrimitiveComponent Object Reference") (OtherBodyIndex :type Integer) (bFromSweep :type Boolean) (SweepResult :type "HitResult Structure (by ref)"))
  (`MovementComponent.StopMovementImmediately` (`self.CharacterMovement`))
  (set `self.IsNotAttacking` false)
  (cast `/Game/Test/BP_PlayerCharacter` OtherActor)
  (if (`self.IsMovingLeft?`)
    (`PaperFlipbookComponent.SetFlipbook` (`self.Sprite`) (`self.AttackLeft`))
    (`KismetSystemLibrary.Delay` (`PaperFlipbookComponent.GetFlipbookLength` (`self.Sprite`)))
    (set `self.IsNotAttacking` true)
    (else
      (`PaperFlipbookComponent.SetFlipbook` (`self.Sprite`) (`self.AttackRight`))
      (`KismetSystemLibrary.Delay` (`PaperFlipbookComponent.GetFlipbookLength` (`self.Sprite`)))
      (set `self.IsNotAttacking` true))))

(event `self.AttackColLeft.OnComponentBeginOverlap`
  (params (OverlappedComponent :type "PrimitiveComponent Object Reference") (OtherActor :type "Actor Object Reference") (OtherComp :type "PrimitiveComponent Object Reference") (OtherBodyIndex :type Integer) (bFromSweep :type Boolean) (SweepResult :type "HitResult Structure (by ref)"))
  (bind _asbp_player_character (cast `/Game/Test/BP_PlayerCharacter` OtherActor))
  (`/Game/Test/BP_PlayerCharacter.TakeHit` _asbp_player_character 5.0))

(event `self.AttackColRight.OnComponentBeginOverlap`
  (params (OverlappedComponent :type "PrimitiveComponent Object Reference") (OtherActor :type "Actor Object Reference") (OtherComp :type "PrimitiveComponent Object Reference") (OtherBodyIndex :type Integer) (bFromSweep :type Boolean) (SweepResult :type "HitResult Structure (by ref)"))
  (bind _asbp_player_character (cast `/Game/Test/BP_PlayerCharacter` OtherActor))
  (`/Game/Test/BP_PlayerCharacter.TakeHit` _asbp_player_character 5.0))

(event `Die`
  (bind _enemyspawner (`self.EnemySpawner`))
  (`/Engine/EditorBlueprintResources/StandardMacros.DoOnce` false
    (:`Completed`
      (`PaperFlipbookComponent.SetFlipbook` (`self.Sprite`) (`self.DyingAnim`))
      (`GameplayStatics.PlaySoundAtLocation` "/Game/Sounds/Effects/Enemy/EnemyDie.EnemyDie" (`self.K2_GetActorLocation`) (struct) 1.0 1.0 0.0 null null null)
      (`NavMovementComponent.StopActiveMovement` (`self.CharacterMovement`))
      (`|AIMoveTo` self (`self.K2_GetActorLocation`) null
        (:`then`
          (set `CharacterMovementComponent.MaxWalkSpeed` 0.0 (`self.CharacterMovement`))
          (set `/Game/BP/EnemySpawner.EnemyKilled` (+ (`/Game/BP/EnemySpawner.EnemyKilled` _enemyspawner) 1) _enemyspawner)
          (`KismetSystemLibrary.Delay` (`PaperFlipbookComponent.GetFlipbookLength` (`self.Sprite`)))
          (`PaperFlipbookComponent.SetFlipbook` (`self.Sprite`) (`self.DeadAnim`))
          (`KismetSystemLibrary.Delay` 1.5)
          (`self.K2_DestroyActor`))))))

(fn `UserConstructionScript`
  (`parent.UserConstructionScript`)
  (set `CharacterMovementComponent.MaxWalkSpeed` (`KismetMathLibrary.RandomFloatInRange` 200.0 400.0) (`self.CharacterMovement`)))