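; BP_TestEnemy is a flipbook-sprite enemy that chases the player with AIMoveTo, with an IsBoss flag for boss behavior.
; Tick reissues the move, fixes sprite rotation and picks left, right or idle flipbooks from velocity and yaw toward the player.
; Attack overlap hits the player, while BattleMusicSphere fades boss music in and out.
; TakeDamage reduces Health; hits at zero destroy bosses, while non-bosses call Die, which destroys only bosses here.
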(event `self.ReceiveBeginPlay`
  (bind _sprite (`self.Sprite`))
  (bind (_returnvalue_roll _returnvalue_pitch _returnvalue_yaw) (`KismetMathLibrary.BreakRotator` (`KismetMathLibrary.FindLookAtRotation` (`self.K2_GetActorLocation`) (`self.K2_GetActorLocation` (`GameplayStatics.GetPlayerCharacter` 0)))))
  (`|AIMoveTo` self (0.0 0.0 0.0) (cast `/Game/Test/BP_PlayerCharacter` (`GameplayStatics.GetPlayerCharacter` 0) :!pure true)
    (:`then`
      (if (> _returnvalue_yaw 0.0)
        (set `self.IsMovingLeft?` false)
        (`PaperFlipbookComponent.SetFlipbook` _sprite (`self.MovingRight`))
        (else
          (set `self.IsMovingLeft?` true)
          (`PaperFlipbookComponent.SetFlipbook` _sprite (`self.MovingLeft`)))))))

(event `self.ReceiveTick`
  (params (DeltaSeconds :type "Float (single-precision)"))
  (bind (_returnvalue_roll _returnvalue_pitch _returnvalue_yaw) (`KismetMathLibrary.BreakRotator` (`KismetMathLibrary.FindLookAtRotation` (`self.K2_GetActorLocation`) (`self.K2_GetActorLocation` (`GameplayStatics.GetPlayerCharacter` 0)))))
  (`|ExecutionSequence`
    (:`then_0`
      (`SceneComponent.K2_SetWorldRotation` (`self.Sprite`) (struct :`Yaw` 90.0 :`Roll` -30.0) false false)
      (`|AIMoveTo` self (0.0 0.0 0.0) (cast `/Game/Test/BP_PlayerCharacter` (`GameplayStatics.GetPlayerCharacter` 0) :!pure true)))
    (:`then_1`
      (if (> _returnvalue_yaw 0.0)
        (set `self.IsMovingLeft?` false)
        (else
          (set `self.IsMovingLeft?` true))))
    (:`then_2`
      (`self.Movement`))))

(event `self.BattleMusicSphere.OnComponentBeginOverlap`
  (params (OverlappedComponent :type "PrimitiveComponent Object Reference") (OtherActor :type "Actor Object Reference") (OtherComp :type "PrimitiveComponent Object Reference") (OtherBodyIndex :type Integer) (bFromSweep :type Boolean) (SweepResult :type "HitResult Structure (by ref)"))
  (`/Engine/EditorBlueprintResources/StandardMacros.DoOnce` false :!label _label
    (:`Completed`
      (if (`self.IsBoss`)
        (cast `/Game/Test/BP_PlayerCharacter` OtherActor)
        (bind _returnvalue (`GameplayStatics.SpawnSoundAtLocation` "/Game/Sounds/Drums/7_-_PIECE_1_4_BATTLE_Cue.7_-_PIECE_1_4_BATTLE_Cue" (`SceneComponent.K2_GetComponentLocation` (`self.CapsuleComponent`)) (struct) 1.0 1.0 0.0 null null))
        (`/Engine/EditorBlueprintResources/StandardMacros.IsValid` _returnvalue
          (:`Is Valid`
            (`AudioComponent.FadeIn` _returnvalue 5.0 2.0 0.0)
            (set `self.BattleMusic` _returnvalue)))))))

(event `self.ReceiveAnyDamage`
  (params (Damage :type "Float (single-precision)") (DamageType :type "DamageType Object Reference") (InstigatedBy :type "Controller Object Reference") (DamageCauser :type "Actor Object Reference"))
  (`self.TakeDamage` Damage))

(event `self.BattleMusicSphere.OnComponentEndOverlap`
  (params (OverlappedComponent :type "PrimitiveComponent Object Reference") (OtherActor :type "Actor Object Reference") (OtherComp :type "PrimitiveComponent Object Reference") (OtherBodyIndex :type Integer))
  (bind _battlemusic (`self.BattleMusic`))
  (cast `/Game/Test/BP_PlayerCharacter` OtherActor)
  (`/Engine/EditorBlueprintResources/StandardMacros.IsValid` _battlemusic
    (:`Is Valid`
      (`AudioComponent.FadeOut` _battlemusic 5.0 0.0)
      (goto _label :!via `Reset`))))

(event `Die`
  (if (`self.IsBoss`)
    (`self.K2_DestroyActor`)))

(event `self.Attack.OnComponentBeginOverlap`
  (params (OverlappedComponent :type "PrimitiveComponent Object Reference") (OtherActor :type "Actor Object Reference") (OtherComp :type "PrimitiveComponent Object Reference") (OtherBodyIndex :type Integer) (bFromSweep :type Boolean) (SweepResult :type "HitResult Structure (by ref)"))
  (bind _asbp_player_character (cast `/Game/Test/BP_PlayerCharacter` OtherActor))
  (`/Game/Test/BP_PlayerCharacter.TakeHit` _asbp_player_character 50.0))

(fn `Movement`
  (bind _sprite (`self.Sprite`))
  (bind (_returnvalue_roll _returnvalue_pitch _returnvalue_yaw) (`KismetMathLibrary.BreakRotator` (`KismetMathLibrary.FindLookAtRotation` (`self.K2_GetActorLocation`) (`self.K2_GetActorLocation` (`GameplayStatics.GetPlayerCharacter` 0)))))
  (if (or (`self.IsBoss`) (`self.IsNotAttacking`))
    (if (`self.Dead`)
      _
      (elif (> (`KismetMathLibrary.VSize` (`self.GetVelocity`)) 0.0)
        (if (> _returnvalue_yaw 0.0)
          (`PaperFlipbookComponent.SetFlipbook` _sprite (`self.MovingRight`))
          (else
            (`PaperFlipbookComponent.SetFlipbook` _sprite (`self.MovingLeft`))))
        (else
          (`PaperFlipbookComponent.SetFlipbook` (`self.Sprite`) (`self.NotMoving`)))))))

(fn `TakeDamage`
  (params (Damage :type "Float (double-precision)"))
  (bind _returnvalue (`self.K2_GetActorLocation`))
  (if (> (`self.Health`) 0.0)
    (set `self.Health` (- (`self.Health`) Damage))
    (`GameplayStatics.PlaySoundAtLocation` (`self.EnemySound`) _returnvalue (struct) 1.0 1.0 0.0 null null null)
    (`GameplayStatics.PlaySoundAtLocation` "/Game/Sounds/Effects/Enemy/EnemyHurt.EnemyHurt" _returnvalue (struct) 1.0 1.0 0.0 null null null)
    (else
      (set `self.Health` 0.0)
      (if (`self.IsBoss`)
        (`self.K2_DestroyActor`)
        (else
          (`self.Die`))))))

(fn `UserConstructionScript`)